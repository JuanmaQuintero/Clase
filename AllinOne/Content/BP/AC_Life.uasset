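; Life component that tracks health, handles damage and healing, and calls DeathMessage on its owner at zero.
; DoDamage routes AutoHeal or DMG_Heal to healing, otherwise subtracts life, playing montages on the cached player character and adjusting the level's PostProcessVolume as feedback.
; Every hit, even a lethal one, starts a four-second delayed Heal event that restores full life.
; IsDead is never set true, and HealPostDamage adds zero life.
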(event `self.ReceiveBeginPlay`
  (set `self.CurrentLife` (`self.MaxLife`))
  (set `self.IsDead` false)
  (bind _asbp_main_character (cast `/Game/BP/BP_MainCharacter` (`GameplayStatics.GetPlayerPawn` 0)))
  (set `self.As BP Main Character` _asbp_main_character))

(event `Heal`
  (`KismetSystemLibrary.Delay` 4.0)
  (`self.DoDamage` (`self.MaxLife`) null true))

(fn `DoDamage`
  (params (Damage :type "Float (double-precision)") (`Damage type` :type "DamageType Object Reference") (AutoHeal :type Boolean))
  (if AutoHeal
    (set `self.CurrentLife` (`KismetMathLibrary.FClamp` (+ (`self.CurrentLife`) Damage) 0.0 (`self.MaxLife`)) :!label _label)
    (`Character.PlayAnimMontage` (`self.As BP Main Character`) "/Game/Animations/AM_HealAnimation.AM_HealAnimation" 1.0 "None")
    (bind _returnvalue (`GameplayStatics.GetActorOfClass` "/Script/Engine.PostProcessVolume"))
    (set `PostProcessVolume.Settings` (make `PostProcessSettings` :`VignetteIntensity` 0.0) _returnvalue)
    (`KismetSystemLibrary.PrintString` "me cure")
    (elif (== (`GameplayStatics.GetObjectClass` `Damage type`) "/Game/BP/DMG_Heal.DMG_Heal_C")
      (goto _label)
      (else
        (bind _output_get (set `self.CurrentLife` (`KismetMathLibrary.FClamp` (- (`self.CurrentLife`) Damage) 0.0 (`self.MaxLife`))))
        (`Character.PlayAnimMontage` (`self.As BP Main Character`) "/Game/Animations/AM_HitAnimation.AM_HitAnimation" 2.5 "None")
        (`self.Heal`)
        (bind _returnvalue_2 (`GameplayStatics.GetActorOfClass` "/Script/Engine.PostProcessVolume"))
        (set `PostProcessVolume.Settings` (make `PostProcessSettings` :`VignetteIntensity` 0.567197) _returnvalue_2)
        (if (<= _output_get 0.0)
          (set `PostProcessVolume.Settings` (make `PostProcessSettings` :`VignetteIntensity` 1.0) _returnvalue_2)
          (message `/Game/Int/I_Death.Death` (`self.GetOwner`)))))))

(fn `HealPostDamage`
  (`KismetSystemLibrary.PrintString` "Me cure despues de 4 segundos")
  (set `self.CurrentLife` (`KismetMathLibrary.FClamp` (+ (`self.CurrentLife`) 0.0) 0.0 (`self.MaxLife`)))
  (bind _returnvalue (`GameplayStatics.GetActorOfClass` "/Script/Engine.PostProcessVolume"))
  (set `PostProcessVolume.Settings` (make `PostProcessSettings` :`VignetteIntensity` 0.0) _returnvalue)
  (`KismetSystemLibrary.PrintString` "me cure"))