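; BP_ParedesHaciaAbajo is a procedural wall builder that lays out a grid of repeated wall pieces.
; Its Construction Script runs nested loops over NumeroDeParedes and ParedesHaciaArriba, adding ParedLimpia instances spaced by Separacion along Y and Distancia along Z.
; Yaw grows by a half turn per Y step, so neighboring columns face opposite ways.
; The event graph holds only disabled default events, with no runtime logic.
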(fn `UserConstructionScript`
  (for _index (range (+ (`self.Numero de paredes`) 1))
    (for _index_2 (range (+ (`self.Paredes Hacia Arriba`) 1))
      (`InstancedStaticMeshComponent.AddInstance` (`self.ParedLimpia`) (`KismetMathLibrary.MakeTransform` (`KismetMathLibrary.MakeVector` 0.0 (`KismetMathLibrary.Conv_IntToDouble` (* _index (`self.Separacion`))) (`KismetMathLibrary.Conv_IntToDouble` (* _index_2 (`self.Distancia`)))) (`KismetMathLibrary.MakeRotator` 0.0 0.0 (`KismetMathLibrary.Conv_IntToDouble` (* _index 180)))) false))))