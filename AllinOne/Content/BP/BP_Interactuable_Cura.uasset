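; BP_Interactuable_Cura is an interactable, single-use healing item for whichever actor interacts with it.
; Its Interaction event sends HealAmount to the Caller through Apply Damage with the DMG_Heal damage type, then destroys the item.
; Healing travels through the damage pipeline, so the receiver's damage handling is what has to turn it into health.
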(event `/Game/Int/I_Interaction.Interaction`
  (params (Caller :type "Actor Object Reference"))
  (`GameplayStatics.ApplyDamage` Caller (`self.HealAmount`) null null "/Game/BP/DMG_Heal.DMG_Heal_C")
  (`self.K2_DestroyActor`))

(fn `UserConstructionScript`
  (`parent.UserConstructionScript`))