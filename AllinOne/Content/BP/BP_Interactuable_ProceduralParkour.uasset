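; An interactable procedural parkour actor that reveals a row of platforms for half a second when interacted with.
; The construction script adds evenly spaced, rotated mesh instances along local X to the Platform component, each at a random height.
; The actor starts hidden with platform collision off at BeginPlay.
; Interaction enables collision and visibility, then a short delay turns both off again.
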(event `self.ReceiveBeginPlay`
  (`PrimitiveComponent.SetCollisionEnabled` (`self.Platform`) "NoCollision")
  (`self.SetActorHiddenInGame` true))

(event `/Game/Int/I_Interaction.Interaction`
  (params (Caller :type "Actor Object Reference"))
  (`PrimitiveComponent.SetCollisionEnabled` (`self.Platform`) "QueryAndPhysics")
  (`self.SetActorHiddenInGame` false)
  (`KismetSystemLibrary.Delay` 0.5)
  (`PrimitiveComponent.SetCollisionEnabled` (`self.Platform`) "NoCollision")
  (`self.SetActorHiddenInGame` true))

(fn `UserConstructionScript`
  (for _index (range 6)
    (`InstancedStaticMeshComponent.AddInstance` (`self.Platform`) (`KismetMathLibrary.MakeTransform` (`KismetMathLibrary.MakeVector` (`KismetMathLibrary.Conv_IntToDouble` (* _index 585)) 0.0 (`KismetMathLibrary.RandomFloatInRange` 30.0 130.0)) (struct :`Yaw` 90.0)) false)))