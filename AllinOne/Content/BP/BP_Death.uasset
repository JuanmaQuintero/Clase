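; BP_Death is a damaging floor, apparently a lethal liquid, tiled to cover an area.
; The construction script fills the Suelo instanced mesh with a fixed-spacing grid sized by Adelante and AlLado.
; When BP_MainCharacter overlaps Suelo, it takes DMG_Liquid damage and is explicitly kept visible.
; Its movement then stops immediately and switches to Flying mode.
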(event `self.Suelo.OnComponentBeginOverlap`
  (params (OverlappedComponent :type "PrimitiveComponent Object Reference") (OtherActor :type "Actor Object Reference") (OtherComp :type "PrimitiveComponent Object Reference") (OtherBodyIndex :type Integer) (bFromSweep :type Boolean) (SweepResult :type "HitResult Structure (by ref)"))
  (bind _charactermovement (`Character.CharacterMovement` (`self.As BP Main Character`)))
  (bind _asbp_main_character (cast `/Game/BP/BP_MainCharacter` OtherActor))
  (bind _output_get (set `self.As BP Main Character` _asbp_main_character))
  (`GameplayStatics.ApplyDamage` _output_get 100.0 null null "/Game/BP/DMG_Liquid.DMG_Liquid_C")
  (`self.SetActorHiddenInGame` (`self.As BP Main Character`) false)
  ;[1 1 1] ?¿?¿¿
  (`MovementComponent.StopMovementImmediately` _charactermovement)
  (`CharacterMovementComponent.SetMovementMode` _charactermovement "MOVE_Flying" 0))

(fn `UserConstructionScript`
  (for _index (range (+ (`self.Adelante`) 1))
    (for _index_2 (range (+ (`self.Al lado`) 1))
      (`InstancedStaticMeshComponent.AddInstance` (`self.Suelo`) (`KismetMathLibrary.MakeTransform` (`KismetMathLibrary.MakeVector` (`KismetMathLibrary.Conv_IntToDouble` (* _index 407)) (`KismetMathLibrary.Conv_IntToDouble` (* _index_2 407)))) false))))