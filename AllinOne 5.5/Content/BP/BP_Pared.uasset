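; BP_Pared is a procedural wall actor that builds two parallel, opposite-facing rows of wall segments.
; Its construction script adds mesh instances along X using NumeroDeParedes and Separacion, offsetting the second row by Distancia and rotating it 180 degrees.
; Each segment is picked at random from an array that repeats components as weighting, favouring plain walls over two window variants.
; The pick is unseeded, and the event graph is empty.
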(fn `UserConstructionScript`
  (bind _paredventanaenmedio (`self.ParedVentanaEnMedio`))
  (bind _paredlimpia (`self.ParedLimpia`))
  (set `self.Paredes` (`|MakeArray` _paredlimpia _paredlimpia _paredlimpia _paredlimpia _paredlimpia _paredlimpia _paredlimpia _paredlimpia _paredlimpia _paredlimpia _paredventanaenmedio (`self.ParedVentanaDerecha`) _paredventanaenmedio))
  (for _index (range (+ (`self.Numero de paredes`) 1))
    (for _index_2 (range 2)
      (`InstancedStaticMeshComponent.AddInstance` (`|GetArrayItem` (`self.Paredes`) (`KismetMathLibrary.RandomInteger` (`KismetArrayLibrary.Array_Length` (`self.Paredes`)))) (`KismetMathLibrary.MakeTransform` (`KismetMathLibrary.MakeVector` (`KismetMathLibrary.Conv_IntToDouble` (* _index (`self.Separacion`))) (`KismetMathLibrary.Conv_IntToDouble` (* _index_2 (`self.Distancia`)))) (`KismetMathLibrary.MakeRotator` 0.0 0.0 (`KismetMathLibrary.Conv_IntToDouble` (* _index_2 180)))) false))))