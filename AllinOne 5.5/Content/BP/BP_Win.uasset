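; BP_Win is a win trigger actor that ends the run when the main character overlaps its Box.
; On BeginPlay it caches the BP_Hud_manager actor and the player's BP_MainCharacter.
; The overlap prints a debug string, disables the overlapping character's forward movement and sets HasWin on itself and the cached character.
; After a four-second delay, it tells the HUD manager to show the win menu.
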(event `self.ReceiveBeginPlay`
  (bind _returnvalue (`GameplayStatics.GetActorOfClass` "/Game/UI/BP_Hud_manager.BP_Hud_manager_C"))
  (set `self.HUD Manager` _returnvalue)
  (set `self.HasWin` false)
  (bind _asbp_main_character (cast `/Game/BP/BP_MainCharacter` (`GameplayStatics.GetPlayerPawn` 0)))
  (set `self.As BP Main Character` _asbp_main_character))

(event `self.Box.OnComponentBeginOverlap`
  (params (OverlappedComponent :type "PrimitiveComponent Object Reference") (OtherActor :type "Actor Object Reference") (OtherComp :type "PrimitiveComponent Object Reference") (OtherBodyIndex :type Integer) (bFromSweep :type Boolean) (SweepResult :type "HitResult Structure (by ref)"))
  (`KismetSystemLibrary.PrintString` "gane")
  (bind _asbp_main_character (cast `/Game/BP/BP_MainCharacter` OtherActor))
  (set `/Game/BP/BP_MainCharacter.ActivateForewardMovement` false _asbp_main_character)
  (bind _output_get (set `self.HasWin` true))
  (set `/Game/BP/BP_MainCharacter.HasWin` _output_get (`self.As BP Main Character`))
  (`KismetSystemLibrary.Delay` 4.0)
  (`/Game/UI/BP_Hud_manager.ShowWinMenu` (`self.HUD Manager`)))

(fn `UserConstructionScript`)