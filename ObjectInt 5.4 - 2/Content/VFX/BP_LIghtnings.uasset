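; Ambient lightning effect Blueprint that makes a lightning plane flash repeatedly during play.
; BeginPlay runs an endless loop that waits a random few seconds, then fires the Strike event.
; Strike plays a timeline from the start, writing its curve value to the plane's materials as the Y parameter and a scaled Intensity parameter.
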(event `self.ReceiveBeginPlay`
  (`KismetSystemLibrary.Delay` (`KismetMathLibrary.RandomFloatInRange` 4.0 8.0) :!label _label)
  (`self.Strike`)
  (goto _label))

(event `Strike`
  (bind (_direction _y) (`Timeline|Lighning_strike` :!via `PlayFromStart`)
    (:`Update`
      (`MeshComponent.SetScalarParameterValueOnMaterials` (`self.Lightning_plane`) "Y" _y)
      (`MeshComponent.SetScalarParameterValueOnMaterials` (`self.Lightning_plane`) "Intensity" (* (+ _y 1.0) 50.0)))))

(fn `UserConstructionScript`)