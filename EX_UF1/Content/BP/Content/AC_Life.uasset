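; AC_Life is a life component that tracks an actor's current life, starting it at MaxLife on BeginPlay.
; DoDamage serves both healing and harm: a DMG_Heal damage type adds the amount, and any other type subtracts it.
; The result is clamped between zero and MaxLife, with no death handling or change notification.
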(event `self.ReceiveBeginPlay`
  (set `self.CurrentLife` (`self.MaxLife`)))

(fn `Do Damage`
  (params (Damage :type "Float (double-precision)") (DamageType :type "DamageType Object Reference"))
  (if (== (`GameplayStatics.GetObjectClass` DamageType) "/Game/BP/Content/DMG_Heal.DMG_Heal_C")
    (set `self.CurrentLife` (`KismetMathLibrary.FClamp` (+ (`self.CurrentLife`) Damage) 0.0 (`self.MaxLife`)))
    (else
      (set `self.CurrentLife` (`KismetMathLibrary.FClamp` (- (`self.CurrentLife`) Damage) 0.0 (`self.MaxLife`))))))